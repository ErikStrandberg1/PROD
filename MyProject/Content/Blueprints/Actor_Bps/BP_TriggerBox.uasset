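; BP_TriggerBox is a trigger actor that halts the player and presents a choice of movement directions.
; Its Box overlap raises OnTriggerOverlap, which disables the Player's character movement, then calls MakeChoice and MovePlayer.
; MakeChoice only prints a left, right or forward prompt matching the AvailableOptions enum.
; No input is read: MovePlayer always receives the same hardcoded enum value, and its body is not shown here.
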(event `self.Box.OnComponentBeginOverlap`
  (params (OverlappedComponent :type "PrimitiveComponent Object Reference") (OtherActor :type "Actor Object Reference") (OtherComp :type "PrimitiveComponent Object Reference") (OtherBodyIndex :type Integer) (bFromSweep :type Boolean) (SweepResult :type "HitResult Structure (by ref)"))
  (if true
    (`self.OnTriggerOverlap` self (`self.Available Options`) (`self.Player`))))

(event `/Game/Blueprints/Interfaces/BPI_Overlapping.OnTriggerOverlap`
  (params (AvailableOptions :type "/Game/Blueprints/ENUM_Directions Enum" :default "NewEnumerator0") (Player :type "/Game/Characters/Charcter/Player Object Reference"))
  (`CharacterMovementComponent.DisableMovement` (`Character.CharacterMovement` Player))
  (`self.MakeChoice`)
  (`/Game/Blueprints/Interfaces/BPI_Overlapping.MovePlayer` self "NewEnumerator1"))

(event `MakeChoice`
  (bind _available_options (`self.Available Options`))
  (if (`|EnumEquality` _available_options "NewEnumerator0")
    (`KismetSystemLibrary.PrintString` "Want to move left or right?")
    (elif (`|EnumEquality` _available_options "NewEnumerator1")
      (`KismetSystemLibrary.PrintString` "Want to move Left or forward?")
      (elif (`|EnumEquality` _available_options "NewEnumerator2")
        (`KismetSystemLibrary.PrintString` "Want to move Right or Forward")))))

(fn `UserConstructionScript`)